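; Player character Blueprint that stubs out a large set of named combo moves, each bound to its own Input Action event.
; Some combo events print debug text on Completed, either a generic test message or a Pure Strength, Speed or Feint label.
; The remaining combo events are empty, and no gameplay logic, BeginPlay, Tick or construction behavior is implemented in this graph.
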(event `EnhancedInput|/Game/_Game/Blueprints/Input/Combos/IA_TestCombo`
  (params (ActionValue :type Boolean) (ElapsedSeconds :type "Float (double-precision)") (TriggeredSeconds :type "Float (double-precision)") (InputAction :type "InputAction Object Reference" :default "/Game/_Game/Blueprints/Input/Combos/IA_TestCombo.IA_TestCombo")))

(event `EnhancedInput|/Game/_Game/Blueprints/Input/Combos/SpeedCombos/IA_Combo_FosterCrs`
  (params (ActionValue :type Boolean) (ElapsedSeconds :type "Float (double-precision)") (TriggeredSeconds :type "Float (double-precision)") (InputAction :type "InputAction Object Reference" :default "/Game/_Game/Blueprints/Input/Combos/SpeedCombos/IA_Combo_FosterCrs.IA_Combo_FosterCrs"))
  (:`Completed`
    (`KismetSystemLibrary.PrintString` "test combo activated")))

(event `EnhancedInput|/Game/_Game/Blueprints/Input/Combos/FeintCombos/IA_Combo_LayerCrs`
  (params (ActionValue :type Boolean) (ElapsedSeconds :type "Float (double-precision)") (TriggeredSeconds :type "Float (double-precision)") (InputAction :type "InputAction Object Reference" :default "/Game/_Game/Blueprints/Input/Combos/FeintCombos/IA_Combo_LayerCrs.IA_Combo_LayerCrs")))

(event `EnhancedInput|/Game/_Game/Blueprints/Input/Combos/StrengthCombos/IA_Combo_StrTailCrs`
  (params (ActionValue :type Boolean) (ElapsedSeconds :type "Float (double-precision)") (TriggeredSeconds :type "Float (double-precision)") (InputAction :type "InputAction Object Reference" :default "/Game/_Game/Blueprints/Input/Combos/StrengthCombos/IA_Combo_StrTailCrs.IA_Combo_StrTailCrs")))

(event `EnhancedInput|/Game/_Game/Blueprints/Input/Combos/SpecialCombos/IA_Combo_Contraband`
  (params (ActionValue :type Boolean) (ElapsedSeconds :type "Float (double-precision)") (TriggeredSeconds :type "Float (double-precision)") (InputAction :type "InputAction Object Reference" :default "/Game/_Game/Blueprints/Input/Combos/SpecialCombos/IA_Combo_Contraband.IA_Combo_Contraband")))

(event `EnhancedInput|/Game/_Game/Blueprints/Input/Combos/StrengthCombos/IA_Combo_PumpFnt`
  (params (ActionValue :type Boolean) (ElapsedSeconds :type "Float (double-precision)") (TriggeredSeconds :type "Float (double-precision)") (InputAction :type "InputAction Object Reference" :default "/Game/_Game/Blueprints/Input/Combos/StrengthCombos/IA_Combo_PumpFnt.IA_Combo_PumpFnt"))
  (:`Completed`
    (`KismetSystemLibrary.PrintString` "test combo activated")))

(event `EnhancedInput|/Game/_Game/Blueprints/Input/Combos/StrengthCombos/IA_Combo_StrTailFnt`
  (params (ActionValue :type Boolean) (ElapsedSeconds :type "Float (double-precision)") (TriggeredSeconds :type "Float (double-precision)") (InputAction :type "InputAction Object Reference" :default "/Game/_Game/Blueprints/Input/Combos/StrengthCombos/IA_Combo_StrTailFnt.IA_Combo_StrTailFnt")))

(event `EnhancedInput|/Game/_Game/Blueprints/Input/Combos/StrengthCombos/IA_Combo_PumpCrs`
  (params (ActionValue :type Boolean) (ElapsedSeconds :type "Float (double-precision)") (TriggeredSeconds :type "Float (double-precision)") (InputAction :type "InputAction Object Reference" :default "/Game/_Game/Blueprints/Input/Combos/StrengthCombos/IA_Combo_PumpCrs.IA_Combo_PumpCrs"))
  (:`Completed`
    (`KismetSystemLibrary.PrintString` "test combo activated")))

(event `EnhancedInput|/Game/_Game/Blueprints/Input/Combos/SpeedCombos/IA_Combo_FosterFnt`
  (params (ActionValue :type Boolean) (ElapsedSeconds :type "Float (double-precision)") (TriggeredSeconds :type "Float (double-precision)") (InputAction :type "InputAction Object Reference" :default "/Game/_Game/Blueprints/Input/Combos/SpeedCombos/IA_Combo_FosterFnt.IA_Combo_FosterFnt"))
  (:`Completed`
    (`KismetSystemLibrary.PrintString` "test combo activated")))

(event `EnhancedInput|/Game/_Game/Blueprints/Input/Combos/FeintCombos/IA_Combo_LayerSpd`
  (params (ActionValue :type Boolean) (ElapsedSeconds :type "Float (double-precision)") (TriggeredSeconds :type "Float (double-precision)") (InputAction :type "InputAction Object Reference" :default "/Game/_Game/Blueprints/Input/Combos/FeintCombos/IA_Combo_LayerSpd.IA_Combo_LayerSpd")))

(event `EnhancedInput|/Game/_Game/Blueprints/Input/Combos/SpecialCombos/IA_Combo_StereotypeX`
  (params (ActionValue :type Boolean) (ElapsedSeconds :type "Float (double-precision)") (TriggeredSeconds :type "Float (double-precision)") (InputAction :type "InputAction Object Reference" :default "/Game/_Game/Blueprints/Input/Combos/SpecialCombos/IA_Combo_StereotypeX.IA_Combo_StereotypeX")))

(event `EnhancedInput|/Game/_Game/Blueprints/Input/Combos/StrengthCombos/IA_Combo_PureStrength`
  (params (ActionValue :type Boolean) (ElapsedSeconds :type "Float (double-precision)") (TriggeredSeconds :type "Float (double-precision)") (InputAction :type "InputAction Object Reference" :default "/Game/_Game/Blueprints/Input/Combos/StrengthCombos/IA_Combo_PureStrength.IA_Combo_PureStrength"))
  (:`Completed`
    (`KismetSystemLibrary.PrintString` "Pure Strength Combo")))

(event `EnhancedInput|/Game/_Game/Blueprints/Input/Combos/StrengthCombos/IA_Combo_PumpSpd`
  (params (ActionValue :type Boolean) (ElapsedSeconds :type "Float (double-precision)") (TriggeredSeconds :type "Float (double-precision)") (InputAction :type "InputAction Object Reference" :default "/Game/_Game/Blueprints/Input/Combos/StrengthCombos/IA_Combo_PumpSpd.IA_Combo_PumpSpd"))
  (:`Completed`
    (`KismetSystemLibrary.PrintString` "test combo activated")))

(event `EnhancedInput|/Game/_Game/Blueprints/Input/Combos/StrengthCombos/IA_Combo_StrTailSpd`
  (params (ActionValue :type Boolean) (ElapsedSeconds :type "Float (double-precision)") (TriggeredSeconds :type "Float (double-precision)") (InputAction :type "InputAction Object Reference" :default "/Game/_Game/Blueprints/Input/Combos/StrengthCombos/IA_Combo_StrTailSpd.IA_Combo_StrTailSpd")))

(event `EnhancedInput|/Game/_Game/Blueprints/Input/Combos/FeintCombos/IA_Combo_LayerStr`
  (params (ActionValue :type Boolean) (ElapsedSeconds :type "Float (double-precision)") (TriggeredSeconds :type "Float (double-precision)") (InputAction :type "InputAction Object Reference" :default "/Game/_Game/Blueprints/Input/Combos/FeintCombos/IA_Combo_LayerStr.IA_Combo_LayerStr")))

(event `EnhancedInput|/Game/_Game/Blueprints/Input/Combos/SpeedCombos/IA_Combo_FosterStr`
  (params (ActionValue :type Boolean) (ElapsedSeconds :type "Float (double-precision)") (TriggeredSeconds :type "Float (double-precision)") (InputAction :type "InputAction Object Reference" :default "/Game/_Game/Blueprints/Input/Combos/SpeedCombos/IA_Combo_FosterStr.IA_Combo_FosterStr"))
  (:`Completed`
    (`KismetSystemLibrary.PrintString` "test combo activated")))

(event `EnhancedInput|/Game/_Game/Blueprints/Input/Combos/SpecialCombos/IA_Combo_Nerdcore`
  (params (ActionValue :type Boolean) (ElapsedSeconds :type "Float (double-precision)") (TriggeredSeconds :type "Float (double-precision)") (InputAction :type "InputAction Object Reference" :default "/Game/_Game/Blueprints/Input/Combos/SpecialCombos/IA_Combo_Nerdcore.IA_Combo_Nerdcore")))

(event `EnhancedInput|/Game/_Game/Blueprints/Input/Combos/SpeedCombos/IA_Combo_PureSpeed`
  (params (ActionValue :type Boolean) (ElapsedSeconds :type "Float (double-precision)") (TriggeredSeconds :type "Float (double-precision)") (InputAction :type "InputAction Object Reference" :default "/Game/_Game/Blueprints/Input/Combos/SpeedCombos/IA_Combo_PureSpeed.IA_Combo_PureSpeed"))
  (:`Completed`
    (`KismetSystemLibrary.PrintString` "Pure Speed Combo")))

(event `EnhancedInput|/Game/_Game/Blueprints/Input/Combos/SpecialCombos/IA_Combo_PostIronic`
  (params (ActionValue :type Boolean) (ElapsedSeconds :type "Float (double-precision)") (TriggeredSeconds :type "Float (double-precision)") (InputAction :type "InputAction Object Reference" :default "/Game/_Game/Blueprints/Input/Combos/SpecialCombos/IA_Combo_PostIronic.IA_Combo_PostIronic")))

(event `EnhancedInput|/Game/_Game/Blueprints/Input/Combos/FeintCombos/IA_Combo_PureFeint`
  (params (ActionValue :type Boolean) (ElapsedSeconds :type "Float (double-precision)") (TriggeredSeconds :type "Float (double-precision)") (InputAction :type "InputAction Object Reference" :default "/Game/_Game/Blueprints/Input/Combos/FeintCombos/IA_Combo_PureFeint.IA_Combo_PureFeint"))
  (:`Completed`
    (`KismetSystemLibrary.PrintString` "Pure Feint Combo")))

(event `EnhancedInput|/Game/_Game/Blueprints/Input/Combos/StrengthCombos/IA_Combo_SandwichCrs`
  (params (ActionValue :type Boolean) (ElapsedSeconds :type "Float (double-precision)") (TriggeredSeconds :type "Float (double-precision)") (InputAction :type "InputAction Object Reference" :default "/Game/_Game/Blueprints/Input/Combos/StrengthCombos/IA_Combo_SandwichCrs.IA_Combo_SandwichCrs"))
  (:`Completed`
    (`KismetSystemLibrary.PrintString` "test combo activated")))

(event `EnhancedInput|/Game/_Game/Blueprints/Input/Combos/SpeedCombos/IA_Combo_WindCrs`
  (params (ActionValue :type Boolean) (ElapsedSeconds :type "Float (double-precision)") (TriggeredSeconds :type "Float (double-precision)") (InputAction :type "InputAction Object Reference" :default "/Game/_Game/Blueprints/Input/Combos/SpeedCombos/IA_Combo_WindCrs.IA_Combo_WindCrs"))
  (:`Completed`
    (`KismetSystemLibrary.PrintString` "test combo activated")))

(event `EnhancedInput|/Game/_Game/Blueprints/Input/Combos/FeintCombos/IA_Combo_DanceCrs`
  (params (ActionValue :type Boolean) (ElapsedSeconds :type "Float (double-precision)") (TriggeredSeconds :type "Float (double-precision)") (InputAction :type "InputAction Object Reference" :default "/Game/_Game/Blueprints/Input/Combos/FeintCombos/IA_Combo_DanceCrs.IA_Combo_DanceCrs")))

(event `EnhancedInput|/Game/_Game/Blueprints/Input/Combos/SpeedCombos/IA_Combo_SpdTailCrs`
  (params (ActionValue :type Boolean) (ElapsedSeconds :type "Float (double-precision)") (TriggeredSeconds :type "Float (double-precision)") (InputAction :type "InputAction Object Reference" :default "/Game/_Game/Blueprints/Input/Combos/SpeedCombos/IA_Combo_SpdTailCrs.IA_Combo_SpdTailCrs")))

(event `EnhancedInput|/Game/_Game/Blueprints/Input/Combos/StrengthCombos/IA_Combo_SandwichFnt`
  (params (ActionValue :type Boolean) (ElapsedSeconds :type "Float (double-precision)") (TriggeredSeconds :type "Float (double-precision)") (InputAction :type "InputAction Object Reference" :default "/Game/_Game/Blueprints/Input/Combos/StrengthCombos/IA_Combo_SandwichFnt.IA_Combo_SandwichFnt"))
  (:`Completed`
    (`KismetSystemLibrary.PrintString` "test combo activated")))

(event `EnhancedInput|/Game/_Game/Blueprints/Input/Combos/SpecialCombos/IA_Combo_SmthFishy`
  (params (ActionValue :type Boolean) (ElapsedSeconds :type "Float (double-precision)") (TriggeredSeconds :type "Float (double-precision)") (InputAction :type "InputAction Object Reference" :default "/Game/_Game/Blueprints/Input/Combos/SpecialCombos/IA_Combo_SmthFishy.IA_Combo_SmthFishy")))

(event `EnhancedInput|/Game/_Game/Blueprints/Input/Combos/SpeedCombos/IA_Combo_WindFnt`
  (params (ActionValue :type Boolean) (ElapsedSeconds :type "Float (double-precision)") (TriggeredSeconds :type "Float (double-precision)") (InputAction :type "InputAction Object Reference" :default "/Game/_Game/Blueprints/Input/Combos/SpeedCombos/IA_Combo_WindFnt.IA_Combo_WindFnt"))
  (:`Completed`
    (`KismetSystemLibrary.PrintString` "test combo activated")))

(event `EnhancedInput|/Game/_Game/Blueprints/Input/Combos/FeintCombos/IA_Combo_DanceSpd`
  (params (ActionValue :type Boolean) (ElapsedSeconds :type "Float (double-precision)") (TriggeredSeconds :type "Float (double-precision)") (InputAction :type "InputAction Object Reference" :default "/Game/_Game/Blueprints/Input/Combos/FeintCombos/IA_Combo_DanceSpd.IA_Combo_DanceSpd")))

(event `EnhancedInput|/Game/_Game/Blueprints/Input/Combos/SpeedCombos/IA_Combo_SpdTailFnt`
  (params (ActionValue :type Boolean) (ElapsedSeconds :type "Float (double-precision)") (TriggeredSeconds :type "Float (double-precision)") (InputAction :type "InputAction Object Reference" :default "/Game/_Game/Blueprints/Input/Combos/SpeedCombos/IA_Combo_SpdTailFnt.IA_Combo_SpdTailFnt")))

(event `EnhancedInput|/Game/_Game/Blueprints/Input/Combos/StrengthCombos/IA_Combo_SandwichSpd`
  (params (ActionValue :type Boolean) (ElapsedSeconds :type "Float (double-precision)") (TriggeredSeconds :type "Float (double-precision)") (InputAction :type "InputAction Object Reference" :default "/Game/_Game/Blueprints/Input/Combos/StrengthCombos/IA_Combo_SandwichSpd.IA_Combo_SandwichSpd"))
  (:`Completed`
    (`KismetSystemLibrary.PrintString` "test combo activated")))

(event `EnhancedInput|/Game/_Game/Blueprints/Input/Combos/FeintCombos/IA_Combo_DanceStr`
  (params (ActionValue :type Boolean) (ElapsedSeconds :type "Float (double-precision)") (TriggeredSeconds :type "Float (double-precision)") (InputAction :type "InputAction Object Reference" :default "/Game/_Game/Blueprints/Input/Combos/FeintCombos/IA_Combo_DanceStr.IA_Combo_DanceStr")))

(event `EnhancedInput|/Game/_Game/Blueprints/Input/Combos/SpeedCombos/IA_Combo_WindStr`
  (params (ActionValue :type Boolean) (ElapsedSeconds :type "Float (double-precision)") (TriggeredSeconds :type "Float (double-precision)") (InputAction :type "InputAction Object Reference" :default "/Game/_Game/Blueprints/Input/Combos/SpeedCombos/IA_Combo_WindStr.IA_Combo_WindStr"))
  (:`Completed`
    (`KismetSystemLibrary.PrintString` "test combo activated")))

(event `EnhancedInput|/Game/_Game/Blueprints/Input/Combos/SpeedCombos/IA_Combo_SpdTailStr`
  (params (ActionValue :type Boolean) (ElapsedSeconds :type "Float (double-precision)") (TriggeredSeconds :type "Float (double-precision)") (InputAction :type "InputAction Object Reference" :default "/Game/_Game/Blueprints/Input/Combos/SpeedCombos/IA_Combo_SpdTailStr.IA_Combo_SpdTailStr")))

(event `EnhancedInput|/Game/_Game/Blueprints/Input/Combos/SpecialCombos/IA_Combo_AsHeTaught`
  (params (ActionValue :type Boolean) (ElapsedSeconds :type "Float (double-precision)") (TriggeredSeconds :type "Float (double-precision)") (InputAction :type "InputAction Object Reference" :default "/Game/_Game/Blueprints/Input/Combos/SpecialCombos/IA_Combo_AsHeTaught.IA_Combo_AsHeTaught")))

(event `EnhancedInput|/Game/_Game/Blueprints/Input/Combos/SpecialCombos/IA_Combo_AdorableExpr`
  (params (ActionValue :type Boolean) (ElapsedSeconds :type "Float (double-precision)") (TriggeredSeconds :type "Float (double-precision)") (InputAction :type "InputAction Object Reference" :default "/Game/_Game/Blueprints/Input/Combos/SpecialCombos/IA_Combo_AdorableExpr.IA_Combo_AdorableExpr")))

(event `EnhancedInput|/Game/_Game/Blueprints/Input/Combos/FeintCombos/IA_Combo_FntTailCrs`
  (params (ActionValue :type Boolean) (ElapsedSeconds :type "Float (double-precision)") (TriggeredSeconds :type "Float (double-precision)") (InputAction :type "InputAction Object Reference" :default "/Game/_Game/Blueprints/Input/Combos/FeintCombos/IA_Combo_FntTailCrs.IA_Combo_FntTailCrs")))

(event `EnhancedInput|/Game/_Game/Blueprints/Input/Combos/FeintCombos/IA_Combo_FntTailSpd`
  (params (ActionValue :type Boolean) (ElapsedSeconds :type "Float (double-precision)") (TriggeredSeconds :type "Float (double-precision)") (InputAction :type "InputAction Object Reference" :default "/Game/_Game/Blueprints/Input/Combos/FeintCombos/IA_Combo_FntTailSpd.IA_Combo_FntTailSpd")))

(event `EnhancedInput|/Game/_Game/Blueprints/Input/Combos/FeintCombos/IA_Combo_FntTailStr`
  (params (ActionValue :type Boolean) (ElapsedSeconds :type "Float (double-precision)") (TriggeredSeconds :type "Float (double-precision)") (InputAction :type "InputAction Object Reference" :default "/Game/_Game/Blueprints/Input/Combos/FeintCombos/IA_Combo_FntTailStr.IA_Combo_FntTailStr")))

(fn `UserConstructionScript`)