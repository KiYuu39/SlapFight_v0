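; Player controller that sets up the main HUD and quick-time-event input for the player.
; BeginPlay creates WBP_MainHUD, adds it to the viewport, shows the mouse cursor, adds the IMC_QTE Enhanced Input mapping context and clears ComboStart.
; The four directional QTE input events are empty.
; Logic forwarding WASD button press and release to the HUD, plus debug prints and test-button casts, is disconnected and never runs.
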(event `self.ReceiveBeginPlay`
  (bind _returnvalue (`|CreateWidget` "/Game/_Game/Blueprints/UI/WBP_MainHUD.WBP_MainHUD_C"))
  (set `self.HUD` _returnvalue)
  (`UserWidget.AddToViewport` _returnvalue 0)
  (`self.EnableInput` null)
  (set `self.bShowMouseCursor` true)
  (`EnhancedInputSubsystemInterface.AddMappingContext` (pcsubsystem `EnhancedInputLocalPlayerSubsystem` self) "/Game/_Game/Blueprints/Input/IMC_QTE.IMC_QTE" 0 (make `ModifyContextOptions` true))
  (set `self.ComboStart` false))

(event `EnhancedInput|/Game/_Game/Blueprints/Input/Actions/IA_QTE_Up`
  (params (ActionValue :type Boolean) (ElapsedSeconds :type "Float (double-precision)") (TriggeredSeconds :type "Float (double-precision)") (InputAction :type "InputAction Object Reference" :default "/Game/_Game/Blueprints/Input/Actions/IA_QTE_Up.IA_QTE_Up"))
  ; Comment
)

(event `EnhancedInput|/Game/_Game/Blueprints/Input/Actions/IA_QTE_Up`
  (params (ActionValue :type Boolean) (ElapsedSeconds :type "Float (double-precision)") (TriggeredSeconds :type "Float (double-precision)") (InputAction :type "InputAction Object Reference" :default "/Game/_Game/Blueprints/Input/Actions/IA_QTE_Up.IA_QTE_Up"))
  ; Comment
)

(event `EnhancedInput|/Game/_Game/Blueprints/Input/Actions/IA_QTE_Down`
  (params (ActionValue :type Boolean) (ElapsedSeconds :type "Float (double-precision)") (TriggeredSeconds :type "Float (double-precision)") (InputAction :type "InputAction Object Reference" :default "/Game/_Game/Blueprints/Input/Actions/IA_QTE_Down.IA_QTE_Down"))
  ; Comment
)

(event `EnhancedInput|/Game/_Game/Blueprints/Input/Actions/IA_QTE_Left`
  (params (ActionValue :type Boolean) (ElapsedSeconds :type "Float (double-precision)") (TriggeredSeconds :type "Float (double-precision)") (InputAction :type "InputAction Object Reference" :default "/Game/_Game/Blueprints/Input/Actions/IA_QTE_Left.IA_QTE_Left"))
  ; Comment
)

(event `EnhancedInput|/Game/_Game/Blueprints/Input/Actions/IA_QTE_Right`
  (params (ActionValue :type Boolean) (ElapsedSeconds :type "Float (double-precision)") (TriggeredSeconds :type "Float (double-precision)") (InputAction :type "InputAction Object Reference" :default "/Game/_Game/Blueprints/Input/Actions/IA_QTE_Right.IA_QTE_Right"))
  ; Comment
)

(fn `UserConstructionScript`)